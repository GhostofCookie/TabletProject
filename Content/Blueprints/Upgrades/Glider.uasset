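; Glider upgrade actor that launches player 0 into flight and shows a usage bar widget from BeginPlay.
; Starting use applies a launch from normalized Y/Z velocity, sets Flying, and starts a looping timer.
; Each tick adds a LaunchCharacter impulse derived from vertical velocity: capped positive Y, one-third Z, zero X.
; Ending use restores Walking, deactivates the exhaust, clears the timer and destroys the actor.
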(event `self.ReceiveBeginPlay`
  (bind _returnvalue (`|CreateWidget` "/Game/Blueprints/UI/W_UsageBar.W_UsageBar_C"))
  (bind _output_get (set `self.W_Usage` _returnvalue))
  (`UserWidget.AddToViewport` _output_get 0))

(event `/Game/Blueprints/HelperLibraries/BPI_Interact.EndUpgradeUse`
  ;[1 1 1] Jetpack!
  (`CharacterMovementComponent.SetMovementMode` (`Character.CharacterMovement` (`GameplayStatics.GetPlayerCharacter` 0)) "MOVE_Walking" 0)
  (`ActorComponent.Deactivate` (`self.EngineExhaust`))
  (`KismetSystemLibrary.PrintString` "Walking" true true (struct :`R` 0.989766 :`G` 0.043877 :`B` 1.0 :`A` 1.0))
  (`KismetSystemLibrary.K2_ClearAndInvalidateTimerHandle` (stale `/Game/Blueprints/HelperLibraries/BPI_Interact.StartUpgradeUse` _returnvalue_2))
  (`self.K2_DestroyActor`))

(event `/Game/Blueprints/HelperLibraries/BPI_Interact.StartUpgradeUse`
  (bind _returnvalue (`GameplayStatics.GetPlayerCharacter` 0))
  ;[1 1 1] Jetpack!
  (`Character.LaunchCharacter` _returnvalue (`self.Get Initial Launch Velocity` _returnvalue) false false)
  (`CharacterMovementComponent.SetMovementMode` (`Character.CharacterMovement` _returnvalue) "MOVE_Flying" 0)
  (`KismetSystemLibrary.PrintString` "Flying")
  (bind _returnvalue_2 (`KismetSystemLibrary.K2_SetTimerDelegate` (delegate `Deplete Flight Velocity`) 0.25 true)))

(event `Deplete Flight Velocity`
  ;[1 1 1] Jetpack!
  (`Character.LaunchCharacter` (`GameplayStatics.GetPlayerCharacter` 0) (`self.Velocity Modifier` (`self.GetVelocity` (`GameplayStatics.GetPlayerCharacter` 0))) false false))

(fn `Get Initial Launch Velocity`
  (params (self2 :type "Actor Object Reference"))
  (returns (ReturnValue :type "Vector Structure"))
  (locals (`Horizontal Velocity` :type "Float (double-precision)"))
  (bind _returnvalue (`self.GetVelocity` self2))
  (set `self.Flight Velocity` _returnvalue)
  (bind _output_get (set `local.Horizontal Velocity` (.y (`KismetMathLibrary.Normal` _returnvalue))))
  (return (`KismetMathLibrary.MakeVector` 0.0 (* _output_get (`self.Y Launch Modifier (Multiply)`)) (+ (.z (`KismetMathLibrary.Normal` _returnvalue)) (`self.Z Launch Modifier (Add)`)))))

(fn `UserConstructionScript`)

(fn `Velocity Modifier`
  (params (InVec :type "Vector Structure"))
  (returns (ReturnValue :type "Vector Structure"))
  (locals (Modifier :type "Float (double-precision)"))
  (bind _z (.z InVec))
  (bind _a_very_useful_variable (`self.A very useful Variable`))
  (bind _returnvalue (/ _z 3.0))
  (bind _returnvalue_2 (+ (`KismetMathLibrary.Abs` _z) (* 1e-05 _z)))
  (`KismetSystemLibrary.PrintString` (`KismetStringLibrary.Conv_DoubleToString` _a_very_useful_variable))
  (if (<= _returnvalue_2 _a_very_useful_variable)
    (`KismetSystemLibrary.PrintString` (`KismetStringLibrary.Conv_DoubleToString` _returnvalue_2) true true (struct :`R` 0.083893 :`B` 1.0 :`A` 1.0))
    (return (`KismetMathLibrary.MakeVector` 0.0 _returnvalue_2 _returnvalue))
    (else
      (`KismetSystemLibrary.PrintString` (`KismetStringLibrary.Conv_DoubleToString` _returnvalue) true true (struct :`R` 1.0 :`G` 0.583564 :`A` 1.0))
      (return (`KismetMathLibrary.MakeVector` 0.0 _a_very_useful_variable _returnvalue)))))