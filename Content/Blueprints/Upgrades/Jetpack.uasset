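; Jetpack upgrade actor that launches the player character upward and sets it to Flying movement, with rocket sound and engine exhaust effects.
; A looping timer drains fuel, updates a usage bar widget created at BeginPlay and applies small upward launches to sustain lift.
; Running out of fuel or ending use restores Walking, clears the timer, removes the upgrade's widgets and destroys the actor, making it single-use.
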(event `self.ReceiveBeginPlay`
  (bind _returnvalue (`|CreateWidget` "/Game/Blueprints/UI/W_UsageBar.W_UsageBar_C"))
  (bind _output_get (set `self.W_Usage` _returnvalue))
  (`UserWidget.AddToViewport` _output_get 0))

(event `/Game/Blueprints/HelperLibraries/BPI_Interact.StartUpgradeUse`
  (bind _returnvalue (`GameplayStatics.GetPlayerCharacter` 0))
  (bind _charactermovement (`Character.CharacterMovement` _returnvalue))
  ;[1 1 1] Jetpack!
  ;;[1 1 1] Play Sound Effect
  (`GameplayStatics.PlaySoundAtLocation` "/Game/Sounds/rocket.rocket" (`SceneComponent.K2_GetComponentLocation` (`MovementComponent.UpdatedPrimitive` _charactermovement)) (struct) 1.0 1.0 0.0 null null null)
  (`Character.LaunchCharacter` _returnvalue (0.0 0.0 500.0) false false)
  (`CharacterMovementComponent.SetMovementMode` _charactermovement "MOVE_Flying" 0)
  (`ActorComponent.Activate` (`self.EngineExhaust`) false)
  (`ActorComponent.Activate` (`self.EngineExhaust2`) false)
  (bind _returnvalue_2 (`KismetSystemLibrary.K2_SetTimerDelegate` (delegate `DepleteFuel`) 0.05 true)))

(event `/Game/Blueprints/HelperLibraries/BPI_Interact.EndUpgradeUse`
  ;[1 1 1] Jetpack!
  (`CharacterMovementComponent.SetMovementMode` (`Character.CharacterMovement` (`GameplayStatics.GetPlayerCharacter` 0)) "MOVE_Walking" 0 :!label _label)
  (`ActorComponent.Deactivate` (`self.EngineExhaust`))
  (`ActorComponent.Deactivate` (`self.EngineExhaust`))
  (`KismetSystemLibrary.K2_ClearAndInvalidateTimerHandle` (stale `/Game/Blueprints/HelperLibraries/BPI_Interact.StartUpgradeUse` _returnvalue_2))
  (`Widget.RemoveFromParent` (`self.W_Usage`))
  (`Widget.RemoveFromParent` (`self.W_UseBtn`))
  (`self.K2_DestroyActor`))

(event `DepleteFuel`
  (bind _w_usage (`self.W_Usage`))
  ;[1 1 1] Jetpack!
  (set `/Game/Blueprints/UI/W_UsageBar.Current` (`self.CurrentFuel`) _w_usage)
  (set `/Game/Blueprints/UI/W_UsageBar.Max` (`self.Fuel Capacity`) _w_usage)
  (bind _output_get (set `self.CurrentFuel` (- (`self.CurrentFuel`) (`self.Depletion Rate`))))
  (if (<= _output_get 0.0)
    (goto _label)
    (else
      (`Character.LaunchCharacter` (`GameplayStatics.GetPlayerCharacter` 0) (0.0 0.0 48.0) false false))))

(fn `UserConstructionScript`)