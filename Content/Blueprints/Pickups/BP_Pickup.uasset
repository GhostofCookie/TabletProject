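; Pickup actor that can be held and dropped, with a data-driven mesh, a radius-sized collision sphere and a camera-facing icon above it.
; Pickup Interface events record the owner and held state and show debug messages.
; HandlePickup snaps it to the owner's ItemSocket and disables mesh collision, or detaches it without restoring collision.
; Looping timers, rather than Tick, drive the icon billboarding and a second event.
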(event `self.ReceiveBeginPlay`
  (`KismetSystemLibrary.K2_SetTimer` null "RotateToCamera" 0.1 true)
  (`KismetSystemLibrary.K2_SetTimerDelegate` (`|CreateDelegate` :!event `HandlePickup`) 0.1 true))

(event `HandlePickup`
  (if (`self.bIsPickedUp`)
    (`self.K2_AttachToActor` (`self.OwningActor`) "ItemSocket" "SnapToTarget" "SnapToTarget" "SnapToTarget")
    (`PrimitiveComponent.SetCollisionEnabled` (`self.Mesh`) "NoCollision")
    (`/Game/Blueprints/ML_HelperMacros.DisplayMessage` "ITEM IS HELD!" (struct :`G` 1.0 :`B` 0.957014 :`A` 1.0))
    (else
      (`/Engine/EditorBlueprintResources/StandardMacros.IsValid` (`self.OwningActor`)
        (:`Is Valid`
          (`self.K2_DetachFromActor` "KeepWorld" "KeepWorld" "KeepWorld")
          (set `self.OwningActor` null))))))

(event `/Game/Blueprints/BPI_Interact.BeginPickup`
  (params (Actor :type "Actor Object Reference"))
  ;[0 0 0] Pickup Interface events
  (set `self.OwningActor` Actor)
  (set `self.bIsPickedUp` true)
  (`/Game/Blueprints/ML_HelperMacros.DisplayMessage` "PICKED UP ITEM!" (struct :`G` 1.0 :`B` 0.026792 :`A` 1.0)))

(event `/Game/Blueprints/BPI_Interact.EndPickup`
  ;[0 0 0] Pickup Interface events
  (set `self.bIsPickedUp` false)
  (`/Game/Blueprints/ML_HelperMacros.DisplayMessage` "DROPPED ITEM!" (struct :`R` 1.0 :`B` 0.039068 :`A` 1.0)))

(fn `RotateToCamera`
  (bind _icon (`self.Icon`))
  (`SceneComponent.K2_SetWorldRotation` _icon (`KismetMathLibrary.Conv_VectorToRotator` (`KismetMathLibrary.GreaterGreater_VectorRotator` (`KismetMathLibrary.Normal` (- (`SceneComponent.K2_GetComponentLocation` (`PlayerCameraManager.TransformComponent` (`GameplayStatics.GetPlayerCameraManager` 0))) (`SceneComponent.K2_GetComponentLocation` _icon))) (struct :`Yaw` 1.0))) false false))

(fn `UserConstructionScript`
  (`|ExecutionSequence`
    (:`then_0`
      (`SphereComponent.SetSphereRadius` (`self.CollisionSphere`) (`self.CollisionRadius`) true))
    (:`then_1`
      (`StaticMeshComponent.SetStaticMesh` (`self.Mesh`) (`.Mesh_11_B5A9B0A44CF6D0A2E9F050AD2C53A675` (break `/Game/Blueprints/Pickups/S_PickupInfo` (`self.PickupInfo`)))))
    (:`then_2`
      (`SceneComponent.K2_SetRelativeLocation` (`self.Icon`) (`KismetMathLibrary.MakeVector` 0.0 0.0 (* (`self.CollisionRadius`) 2.0)) false false))))