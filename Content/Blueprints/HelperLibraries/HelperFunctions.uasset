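; Blueprint helper library of small general-purpose utility functions.
; TextToName converts text to a Name by way of a string.
; The actor and widget lookups gather all instances of a given class and return element zero without checking for an empty result.
; The widget search also includes nested widgets, not just top-level ones.
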(fn `GetFirstActorOfClass`
  (params (ActorClass :type "Actor Class Reference"))
  (returns (Actor :type "Actor Object Reference"))
  (bind _outactors (`GameplayStatics.GetAllActorsOfClass` null ActorClass))
  (return (`|GetArrayItem` _outactors)))

(fn `GetFirstWidgetOfClass`
  (params (ActorClass :type "UserWidget Class Reference"))
  (returns (Widget :type "UserWidget Object Reference"))
  (bind _foundwidgets (`WidgetBlueprintLibrary.GetAllWidgetsOfClass` null ActorClass false))
  (return (`|GetArrayItem` _foundwidgets)))

(fn `TextToName`
  (params (In :type Text))
  (returns (Out :type Name))
  (return (`KismetStringLibrary.Conv_StringToName` (`KismetTextLibrary.Conv_TextToString` In))))