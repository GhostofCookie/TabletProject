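; BP_TrashCan is a trash can actor that interrupts play so the player can toss trash.
; When BP_TopDownCharacter overlaps TriggerGarbagePause, it tells the first BP_dball in the level to stop and starts a camera fade out.
; After a short delay it adds the W_TrashMenu widget to the viewport and clears the fade.
; Nothing in this Blueprint restarts the ball.
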(event `self.triggerGarbagePause.OnComponentBeginOverlap`
  (params (OverlappedComponent :type "PrimitiveComponent Object Reference") (OtherActor :type "Actor Object Reference") (OtherComp :type "PrimitiveComponent Object Reference") (OtherBodyIndex :type Integer) (bFromSweep :type Boolean) (SweepResult :type "HitResult Structure (by ref)"))
  ;[1 1 1] cast to only recognize player
  (cast `/Game/Blueprints/Player/BP_TopDownCharacter` OtherActor)
  ;[1 1 1] add at end to start ball again
  (bind _actor (`/Game/Blueprints/HelperLibraries/HelperFunctions.GetFirstActorOfClass` "/Game/Blueprints/hazards/BP_d-ball.BP_d-ball_C"))
  (bind _asbp_d_ball (cast `/Game/Blueprints/hazards/BP_d-ball` _actor))
  (`/Game/Blueprints/hazards/BP_d-ball.StopBall` _asbp_d_ball)
  ;[1 1 1] FADE
  (`PlayerCameraManager.StartCameraFade` :`self` (`GameplayStatics.GetPlayerCameraManager` 0) :`ToAlpha` 1.0 :`Duration` 2.0 :`bHoldWhenFinished` true)
  (`KismetSystemLibrary.Delay` 2.5)
  ;[1 1 1] open menu to toss trash
  (bind _returnvalue (`|CreateWidget` "/Game/Blueprints/UI/W_TrashMenu.W_TrashMenu_C"))
  (`UserWidget.AddToViewport` _returnvalue 0)
  (`PlayerCameraManager.StopCameraFade` (`GameplayStatics.GetPlayerCameraManager` 0)))

(fn `UserConstructionScript`)