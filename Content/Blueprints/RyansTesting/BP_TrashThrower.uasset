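; BP_TrashThrower spawns a batch of six child garbage actors at random points inside SpawnArea and flings them with physics.
; Each Tick applies a Y/Z acceleration to every BP_Garbage mesh, decrementing the shared force per piece and resetting it near the negated start value.
; A five-second Delay on Tick restores the starting force, destroys the batch and spawns another; the construction script creates the first.
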(event `/Game/Blueprints/BPI_Interact.Reset`
  ;[1 0 0] RESET on death, however Dont think this is needed because clear and spawn is handled on tick anyway
)

(event `self.ReceiveTick`
  (params (DeltaSeconds :type "Float (single-precision)"))
  (`|ExecutionSequence`
    (:`then_0`
      (`KismetSystemLibrary.Delay` 5.0)
      (set `self.currentY` (`self.startY`))
      (set `self.currentZ` (`self.startZ`))
      (`self.ClearItems`)
      (`self.SpawnTrash`))
    (:`then_1`
      (for _array_element (`self.GetAllChildActors` true)
        (`/Engine/EditorBlueprintResources/StandardMacros.IsValid` _array_element
          (:`Is Valid`
            (bind _asbp_garbage (cast `/Game/Blueprints/Pickups/BP_Garbage` _array_element))
            (bind _mesh (`/Game/Blueprints/Pickups/BP_Pickup.Mesh` _asbp_garbage))
            (`PrimitiveComponent.SetSimulatePhysics` _mesh true)
            (`PrimitiveComponent.AddForce` _mesh (`KismetMathLibrary.MakeVector` 0.0 (`self.currentY`) (`self.currentZ`)) "None" true)
            (set `self.currentY` (- (`self.currentY`) 5.0))
            (set `self.currentZ` (- (`self.currentZ`) 5.0))
            (`self.ResetYZvelocity`)))))))

(fn `ClearItems`
  (for _array_element (`self.GetAllChildActors` true)
    (`/Engine/EditorBlueprintResources/StandardMacros.IsValid` _array_element
      (:`Is Valid`
        (`self.K2_DestroyActor` _array_element)))))

(fn `getchildren`
  (returns (Mesh :type "StaticMeshComponent Object Reference"))
  (for _array_element (`self.GetAllChildActors` true)
    (`/Engine/EditorBlueprintResources/StandardMacros.IsValid` _array_element
      (:`Is Valid`
        (bind _asbp_garbage (cast `/Game/Blueprints/Pickups/BP_Garbage` _array_element))
        (bind _mesh (`/Game/Blueprints/Pickups/BP_Pickup.Mesh` _asbp_garbage))
        (`PrimitiveComponent.SetSimulatePhysics` _mesh true)
        (return _mesh))))
  (return _mesh))

(fn `ResetYZvelocity`
  (if (`KismetMathLibrary.NearlyEqual_FloatFloat` (`self.currentY`) (* -1 (`self.startY`)) 6.0)
    (set `self.currentY` (`self.startY`)))
  (if (`KismetMathLibrary.NearlyEqual_FloatFloat` (`self.currentZ`) (* -1 (`self.startZ`)) 6.0)
    (set `self.currentZ` (`self.startZ`))))

(fn `SpawnTrash`
  (bind _spawnarea (`self.SpawnArea`))
  (for _ (range 6)
    (`AddComponent|NODE_AddChildActorComponent-0` :`RelativeTransform` (`KismetMathLibrary.Conv_VectorToTransform` (`KismetMathLibrary.RandomPointInBoundingBox` (`SceneComponent.RelativeLocation` _spawnarea) (`BoxComponent.BoxExtent` _spawnarea))))))

(fn `UserConstructionScript`
  (`self.SpawnTrash`))