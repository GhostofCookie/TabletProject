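; Spawner for a recycling feature that scatters a small batch of child actors at random points inside its Box component.
; The construction script creates the initial batch through AddChildActorComponent, using relative transforms taken from the box bounds.
; A Reset event destroys every valid BP_Recyclable in the world, not just this spawner's own, then spawns a fresh batch.
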(event `/Game/Blueprints/BPI_Interact.Reset`
  (`self.clearItems`)
  (`self.SpawnItems`))

(fn `clearItems`
  (bind _outactors (`GameplayStatics.GetAllActorsOfClass` "/Game/Blueprints/Pickups/BP_Recyclable.BP_Recyclable_C"))
  (for _array_element _outactors
    (`/Engine/EditorBlueprintResources/StandardMacros.IsValid` _array_element
      (:`Is Valid`
        (`self.K2_DestroyActor` _array_element)))))

(fn `SpawnItems`
  (bind _box (`self.Box`))
  (for _ (range 6)
    (`AddComponent|NODE_AddChildActorComponent-0` :`RelativeTransform` (`KismetMathLibrary.Conv_VectorToTransform` (`KismetMathLibrary.RandomPointInBoundingBox` (`SceneComponent.RelativeLocation` _box) (`BoxComponent.BoxExtent` _box))))))

(fn `UserConstructionScript`
  (`self.SpawnItems`))