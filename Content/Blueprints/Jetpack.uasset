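; Jetpack upgrade that lets the first player's character fly while fuel lasts.
; Starting use switches character movement to Flying, activates the engine exhaust and starts a looping timer that drains CurrentFuel by DepletionRate.
; Empty fuel or ending use share one shutdown path that restores Walking, deactivates the exhaust and clears the timer.
; The graph contains no refuel logic and no fuel check on start.
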(event `DepleteFuel`
  ;[1 1 1] Jetpack!
  (bind _output_get (set `self.CurrentFuel` (- (`self.CurrentFuel`) (`self.Depletion Rate`))))
  (if (<= _output_get 0.0)
    (`CharacterMovementComponent.SetMovementMode` (`Character.CharacterMovement` (`GameplayStatics.GetPlayerCharacter` 0)) "MOVE_Walking" 0 :!label _label)
    (`ActorComponent.Deactivate` (`self.EngineExhaust`))
    (`KismetSystemLibrary.K2_ClearAndInvalidateTimerHandle` (stale `/Game/Blueprints/BPI_Interact.StartUpgradeUse` _returnvalue))))

(event `/Game/Blueprints/BPI_Interact.StartUpgradeUse`
  ;[1 1 1] Jetpack!
  (`CharacterMovementComponent.SetMovementMode` (`Character.CharacterMovement` (`GameplayStatics.GetPlayerCharacter` 0)) "MOVE_Flying" 0)
  (`ActorComponent.Activate` (`self.EngineExhaust`) false)
  (bind _returnvalue (`KismetSystemLibrary.K2_SetTimerDelegate` (delegate `DepleteFuel`) 0.05 true)))

(event `/Game/Blueprints/BPI_Interact.EndUpgradeUse`
  ;[1 1 1] Jetpack!
  (goto _label))

(event `self.ReceiveBeginPlay`
  ;[1 1 1] Jetpack!
)

(fn `UserConstructionScript`)