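; BP_SideElevator is a moving platform that travels while the top-down player character is in its trigger.
; On overlap, a short delay precedes a timeline that lerps the Elevator component's relative location from StartLoc to the EndLocation component's relative location.
; When the character leaves the trigger, the timeline reverses from its current point, moving the platform back toward the start.
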(event `self.Trigger.OnComponentBeginOverlap`
  (params (OverlappedComponent :type "PrimitiveComponent Object Reference") (OtherActor :type "Actor Object Reference") (OtherComp :type "PrimitiveComponent Object Reference") (OtherBodyIndex :type Integer) (bFromSweep :type Boolean) (SweepResult :type "HitResult Structure (by ref)"))
  (cast `/Game/Blueprints/Player/BP_TopDownCharacter` OtherActor)
  ;[1 1 1] Delay before boat moves
  (`KismetSystemLibrary.Delay` 0.2)
  (bind (_direction _newtrack_0) (`Timeline|Timeline_0` :!label _label)
    (:`Update`
      (`SceneComponent.K2_SetRelativeLocation` (`self.Elevator`) (`KismetMathLibrary.VLerp` (`self.StartLoc`) (`SceneComponent.RelativeLocation` (`self.EndLocation`)) _newtrack_0) false false))))

(event `self.Trigger.OnComponentEndOverlap`
  (params (OverlappedComponent :type "PrimitiveComponent Object Reference") (OtherActor :type "Actor Object Reference") (OtherComp :type "PrimitiveComponent Object Reference") (OtherBodyIndex :type Integer))
  (cast `/Game/Blueprints/Player/BP_TopDownCharacter` OtherActor)
  (goto _label :!via `Reverse`))

(fn `UserConstructionScript`)