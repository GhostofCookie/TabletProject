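; Recycling center actor that opens its UI when the player walks into it.
; When the player's top-down character overlaps the Enter component, it finds the first deathball actor in the level and calls its StopBall.
; It then creates the W_RecyclingCenter widget, stores the reference and adds it to the viewport.
; The construction script and fadeMacro are empty.
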(event `self.enter.OnComponentBeginOverlap`
  (params (OverlappedComponent :type "PrimitiveComponent Object Reference") (OtherActor :type "Actor Object Reference") (OtherComp :type "PrimitiveComponent Object Reference") (OtherBodyIndex :type Integer) (bFromSweep :type Boolean) (SweepResult :type "HitResult Structure (by ref)"))
  (if (== OtherActor (`GameplayStatics.GetPlayerPawn` 0))
    (cast `/Game/Blueprints/Player/BP_TopDownCharacter` OtherActor)
    ;[1 1 1] Stops ball
    (bind _actor (`/Game/Blueprints/HelperLibraries/HelperFunctions.GetFirstActorOfClass` "/Game/Blueprints/hazards/BP_death-ball.BP_death-ball_C"))
    (bind _asbp_death_ball (cast `/Game/Blueprints/hazards/BP_death-ball` _actor))
    (`/Game/Blueprints/hazards/BP_death-ball.StopBall` _asbp_death_ball)
    ;[1 1 1] Open Widget
    (bind _returnvalue (`|CreateWidget` "/Game/Blueprints/UI/Menus/W_RecyclingCenter.W_RecyclingCenter_C"))
    (set `self.WidgetRef` _returnvalue)
    (`UserWidget.AddToViewport` (`self.WidgetRef`) 0)))

(fn `UserConstructionScript`)