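; Recycling spawner that fills a box volume with small, randomly placed items as child actors.
; The construction script runs SpawnItems, which adds a fixed number of child actor components at random points in the box and shrinks each spawned actor with a temporary scale.
; A Reset event destroys all child actors through ClearItems, then spawns a fresh random set.
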(event `/Game/Blueprints/HelperLibraries/BPI_Interact.Reset`
  (`self.clearItems`)
  (`self.SpawnItems`))

(fn `clearItems`
  (for _array_element (`self.GetAllChildActors` true)
    (`/Engine/EditorBlueprintResources/StandardMacros.IsValid` _array_element
      (:`Is Valid`
        (`self.K2_DestroyActor` _array_element)))))

(fn `SpawnItems`
  (bind _box (`self.Box`))
  (for _ (range 6)
    (bind _returnvalue (`AddComponent|NODE_AddChildActorComponent-0` :`RelativeTransform` (`KismetMathLibrary.Conv_VectorToTransform` (`KismetMathLibrary.RandomPointInBoundingBox` (`SceneComponent.RelativeLocation` _box) (`BoxComponent.BoxExtent` _box)))))
    ;[1 0.09582 0] CHANGE SCALE LATER when models on on
    (`self.SetActorScale3D` (`ChildActorComponent.ChildActor` _returnvalue) (0.25 0.25 0.25))))

(fn `UserConstructionScript`
  (`self.SpawnItems`))