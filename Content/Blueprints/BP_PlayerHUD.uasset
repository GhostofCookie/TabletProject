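; BP_PlayerHUD is a HUD Blueprint that puts the W_Raderv2TomasHelp widget on screen to track the horizontal position of BP_dball.
; BeginPlay creates the widget and adds it to the viewport; a custom show event repeats this, but its binding never runs.
; Every DrawHUD looks up the first BP_dball, projects its location to screen, and shifts the widget to that X with Y fixed at zero.
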(event `self.ReceiveBeginPlay`
  (bind _returnvalue (`|CreateWidget` "/Game/Blueprints/UI/RyansWidgets/W_Raderv2TomasHelp.W_Raderv2TomasHelp_C" :!label _label))
  (`UserWidget.AddToViewport` _returnvalue 0))

(event `ShowPlayerHUD_Event`
  (goto _label))

(event `self.ReceiveDrawHUD`
  (params (SizeX :type Integer) (SizeY :type Integer))
  (bind _actor (`/Game/Blueprints/HelperLibraries/HelperFunctions.GetFirstActorOfClass` "/Game/Blueprints/hazards/BP_d-ball.BP_d-ball_C"))
  (`Widget.SetRenderTranslation` (stale `self.ReceiveBeginPlay` _returnvalue) (`KismetMathLibrary.MakeVector2D` (`KismetMathLibrary.BreakVector2D` (`PlayerController.ProjectWorldLocationToScreen` (`GameplayStatics.GetPlayerController` 0) (`self.K2_GetActorLocation` _actor) false)))))

(fn `UserConstructionScript`)