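; Rolling ball hazard that moves along Y and catches the player, carrying them along with it.
; Tick zeroes the mesh's relative X, adds force while slow, and resets Y velocity once it reaches the character's max speed.
; An Arrow follows the ball at a fixed offset and world rotation, serving as a non-spinning anchor.
; On character overlap, Deathtrigger disables player input, movement and collision, then attaches the capsule to that Arrow.
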(event `self.ReceiveTick`
  (params (DeltaSeconds :type "Float (single-precision)"))
  (bind _ballmesh (`self.BallMesh`))
  (bind _ballmesh_2 (`self.BallMesh`))
  (bind _returnvalue (`MovementComponent.GetMaxSpeed` (`Pawn.GetMovementComponent` (`GameplayStatics.GetPlayerCharacter` 0))))
  (`|ExecutionSequence`
    (:`then_0`
      ;[1 1 1] Ensure ball doesn't fall off
      (`SceneComponent.K2_SetRelativeLocation` _ballmesh_2 (* (`SceneComponent.RelativeLocation` _ballmesh_2) (0.0 1.0 1.0)) false true)
      ;[1 1 1] handles ball velocity and gravity
      (`/Engine/EditorBlueprintResources/StandardMacros.IsValid` (`GameplayStatics.GetPlayerCharacter` 0)
        (:`Is Valid`
          (if (<= (`KismetMathLibrary.Abs` (.y (`SceneComponent.GetComponentVelocity` _ballmesh))) _returnvalue)
            (`PrimitiveComponent.AddForce` _ballmesh (`self.ballImpulse`) "None" true))
          (if (>= (.y (`SceneComponent.GetComponentVelocity` (`self.BallMesh`))) _returnvalue)
            (`PrimitiveComponent.SetPhysicsLinearVelocity` (`self.BallMesh`) (`KismetMathLibrary.MakeVector` 0.0 600.0 (.z (`SceneComponent.GetComponentVelocity` (`self.BallMesh`)))) false "None")))))
    (:`then_1`
      ;[1 1 1] Arrow Rotation to keep constant
      (`SceneComponent.K2_SetWorldRotation` (`self.Arrow`) (`self.StartingRotation`) false false))
    (:`then_2`
      ;[1 1 1] set arrow location to stay with ball
      (`SceneComponent.K2_SetWorldLocation` (`self.Arrow`) (+ (`self.arrowOffset`) (`SceneComponent.K2_GetComponentLocation` (`self.BallMesh`))) true false))))

(event `self.death-trigger.OnComponentBeginOverlap`
  (params (OverlappedComponent :type "PrimitiveComponent Object Reference") (OtherActor :type "Actor Object Reference") (OtherComp :type "PrimitiveComponent Object Reference") (OtherBodyIndex :type Integer) (bFromSweep :type Boolean) (SweepResult :type "HitResult Structure (by ref)"))
  (cast `Character` OtherActor)
  ;[1 1 1] disable input
  (`self.DisableInput` (`GameplayStatics.GetPlayerCharacter` 0) null)
  ;[1 1 1] double check physics is off
  (`PrimitiveComponent.SetSimulatePhysics` (`Character.CapsuleComponent` (`GameplayStatics.GetPlayerCharacter` 0)) false)
  ;[1 1 1] stop movement
  (`MovementComponent.StopMovementImmediately` (`Character.CharacterMovement` (`GameplayStatics.GetPlayerCharacter` 0)))
  ;[1 1 1] Attache to arrow
  (`SceneComponent.K2_AttachToComponent` (`Character.CapsuleComponent` (`GameplayStatics.GetPlayerCharacter` 0)) (`self.Arrow`) "None" "SnapToTarget" "KeepWorld" "KeepWorld" true)
  ;[1 1 1] Turn off collisions
  (`PrimitiveComponent.SetCollisionEnabled` (`Character.CapsuleComponent` (`GameplayStatics.GetPlayerCharacter` 0)) "NoCollision")
  (`PrimitiveComponent.SetCollisionEnabled` (`self.death-trigger`) "NoCollision"))

(event `self.ReceiveBeginPlay`
  ;[1 1 1] sets the variables to keep track oflocation and rotation
  (`|ExecutionSequence`
    (:`then_0`
      (set `self.StartingRotation` (`SceneComponent.K2_GetComponentRotation` (`self.Arrow`)))
      (set `self.arrowOffset` (`SceneComponent.RelativeLocation` (`self.Arrow`))))))

(fn `UserConstructionScript`)