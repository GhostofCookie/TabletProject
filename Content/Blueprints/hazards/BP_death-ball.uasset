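; Death ball hazard: a physics ball that chases the player along Y and kills on overlap.
; Each tick it flips impulse toward the player, caps speed at the character's max, pins X and counters falling.
; An Arrow tracks the player until impact, then the dying character is attached and follows its rotation.
; Start/stop events toggle physics and player input; BeginPlay saves a game-instance checkpoint that Reset reloads.
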(event `self.ReceiveBeginPlay`
  ;[1 1 1] Dispatching
  (add `self.StopBall` (`|CreateDelegate` :!event `StopBall_Event`))
  (add `self.startBall` (`|CreateDelegate` :!event `startBall_Event`))
  (bind _asbp_recycling_game_instance (cast `/Game/Blueprints/BP_RecyclingGameInstance` (`GameplayStatics.GetGameInstance`)))
  (`/Game/Blueprints/BP_RecyclingGameInstance.SaveCheckpoint` _asbp_recycling_game_instance (`self.K2_GetActorLocation`) "TPCP_DB_1"))

(event `StopBall_Event`
  (set `self.StopBallCheck` false)
  (`PrimitiveComponent.SetSimulatePhysics` (`self.Ball`) false)
  (`self.DisableInput` (`GameplayStatics.GetPlayerCharacter` 0) null))

(event `startBall_Event`
  (set `self.StopBallCheck` true)
  (`PrimitiveComponent.SetSimulatePhysics` (`self.Ball`) true)
  (`self.EnableInput` (`GameplayStatics.GetPlayerCharacter` 0) null))

(event `self.ReceiveTick`
  (params (DeltaSeconds :type "Float (single-precision)"))
  (bind _returnvalue (`GameplayStatics.GetPlayerCharacter` 0))
  (bind _arrow (`self.Arrow`))
  (bind _ball (`self.Ball`))
  (bind _returnvalue_2 (`MovementComponent.GetMaxSpeed` (`Pawn.GetMovementComponent` (`GameplayStatics.GetPlayerCharacter` 0))))
  (`|ExecutionSequence`
    (:`then_0`
      (`|ExecutionSequence`
        (:`then_0`
          (if (`self.comparePlayerBallLocation`)
            (`self.setBallMotionBackWard`)
            (else
              (`self.setBallMotionForward`))))
        (:`then_1`
          (if (`self.StopBallCheck`)
            (`/Engine/EditorBlueprintResources/StandardMacros.IsValid` (`GameplayStatics.GetPlayerCharacter` 0)
              (:`Is Valid`
                (`self.PreventBallFall` _ball
                  (:`then`
                    _)
                  (:`OutputPin`
                    _))
                (if (<= (`KismetMathLibrary.Abs` (.y (`SceneComponent.GetComponentVelocity` _ball))) _returnvalue_2)
                  (`PrimitiveComponent.AddForce` _ball (`self.ballImpulse`) "None" true))
                (if (>= (.y (`SceneComponent.GetComponentVelocity` (`self.Ball`))) _returnvalue_2)
                  (`PrimitiveComponent.SetPhysicsLinearVelocity` (`self.Ball`) (`KismetMathLibrary.MakeVector` 0.0 _returnvalue_2 (.z (`SceneComponent.GetComponentVelocity` (`self.Ball`)))) false "None"))))))))
    (:`then_1`
      (if (not (`self.Attached`))
        (`SceneComponent.K2_SetWorldRotation` _arrow (`KismetMathLibrary.Conv_VectorToRotator` (`KismetMathLibrary.GreaterGreater_VectorRotator` (`KismetMathLibrary.Normal` (- (`SceneComponent.K2_GetComponentLocation` (`Actor.RootComponent` (`GameplayStatics.GetPlayerCharacter` 0))) (`SceneComponent.K2_GetComponentLocation` (`self.Arrow`)))) (struct :`Yaw` 1.0))) false false)
        (else
          (`self.K2_SetActorRotation` _returnvalue (`SceneComponent.K2_GetComponentRotation` _arrow) false)
          (`self.K2_SetActorRelativeLocation` _returnvalue (0.0 0.0 0.0) false false))))))

(event `self.death-trigger.OnComponentBeginOverlap`
  (params (OverlappedComponent :type "PrimitiveComponent Object Reference") (OtherActor :type "Actor Object Reference") (OtherComp :type "PrimitiveComponent Object Reference") (OtherBodyIndex :type Integer) (bFromSweep :type Boolean) (SweepResult :type "HitResult Structure (by ref)"))
  (bind _asbp_top_down_character (cast `/Game/Blueprints/Player/BP_TopDownCharacter` OtherActor))
  (`self.DisableInput` _asbp_top_down_character (`GameplayStatics.GetPlayerController` 0))
  (`MovementComponent.StopMovementImmediately` (`Character.CharacterMovement` _asbp_top_down_character))
  (`self.K2_AttachToComponent` _asbp_top_down_character (`self.AttachLocation`) "None" "SnapToTarget" "SnapToTarget" "KeepWorld" true)
  (`PrimitiveComponent.SetCollisionEnabled` (`Character.CapsuleComponent` _asbp_top_down_character) "NoCollision")
  (set `self.Attached` true)
  (`/Game/Blueprints/Player/BP_TopDownCharacter.Death` _asbp_top_down_character))

(event `/Game/Blueprints/HelperLibraries/BPI_Interact.Reset`
  (bind _asbp_recycling_game_instance (cast `/Game/Blueprints/BP_RecyclingGameInstance` (`GameplayStatics.GetGameInstance`))
    (:`then`
      (`/Game/Blueprints/BP_RecyclingGameInstance.LoadCheckpoint` _asbp_recycling_game_instance self "TPCP_DB_1")
      (set `self.Attached` false)
      (`KismetSystemLibrary.PrintString` "Hello"))
    (:`CastFailed`
      (`KismetSystemLibrary.PrintString` "Failed!"))))

(fn `UserConstructionScript`)