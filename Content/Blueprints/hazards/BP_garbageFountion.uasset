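; Garbage fountain hazard that loops the movement of a sludge mesh, with an overlap kill box that currently does nothing.
; BeginPlay stores the sludge's start location, then plays a timeline whose height is added to the current relative Z on every update, so movement accumulates.
; Each update also sets world scale through VectorMultiplier, whose scaling math is unconnected.
; When the timeline finishes, the sludge snaps back to its start and replays.
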(event `self.ReceiveBeginPlay`
  (bind _returnvalue (`self.sludgeHeightAdjuster`))
  ;[1 1 1] loops the scale and movement of the sludge "trash"
  (`|ExecutionSequence`
    (:`then_0`
      (set `self.startLocation` (`SceneComponent.K2_GetComponentLocation` (`self.sludge`))))
    (:`then_1`
      (bind (_direction _height) (`Timeline|Timeline_0` :!label _label)
        (:`Update`
          (set `self.sludge_height` _height)
          (`SceneComponent.SetWorldScale3D` (`self.sludge`) (`KismetMathLibrary.MakeVector` 1.0 1.0 (* (.z _returnvalue) 0.045)))
          (`SceneComponent.K2_SetRelativeLocation` (`self.sludge`) _returnvalue false false))
        (:`Finished`
          (`SceneComponent.K2_SetWorldLocation` (`self.sludge`) (`self.startLocation`) false false)
          (goto _label :!via `PlayFromStart`))))))

(event `self.killBox.OnComponentBeginOverlap`
  (params (OverlappedComponent :type "PrimitiveComponent Object Reference") (OtherActor :type "Actor Object Reference") (OtherComp :type "PrimitiveComponent Object Reference") (OtherBodyIndex :type Integer) (bFromSweep :type Boolean) (SweepResult :type "HitResult Structure (by ref)"))
  ;[1 1 1] death block
)

(fn `sludgeHeightAdjuster`
  (returns (ReturnValue :type "Vector Structure"))
  (return (`KismetMathLibrary.MakeVector` (.x (`SceneComponent.RelativeLocation` (`self.sludge`))) (.y (`SceneComponent.RelativeLocation` (`self.sludge`))) (+ (.z (`SceneComponent.RelativeLocation` (`self.sludge`))) (`self.sludge_height`)))))

(fn `UserConstructionScript`)