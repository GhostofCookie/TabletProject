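; BP_pizzaSlow is a hazard that temporarily slows the player when a Character enters its Box trigger.
; On overlap it sets player 0's MaxWalkSpeed to SlowSpeed, waits SlowDuration, then sets it to NormalSpeed.
; Any Character can trigger it, but the speed change always applies to player 0 rather than the overlapping actor.
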(event `self.Box.OnComponentBeginOverlap`
  (params (OverlappedComponent :type "PrimitiveComponent Object Reference") (OtherActor :type "Actor Object Reference") (OtherComp :type "PrimitiveComponent Object Reference") (OtherBodyIndex :type Integer) (bFromSweep :type Boolean) (SweepResult :type "HitResult Structure (by ref)"))
  (cast `Character` OtherActor)
  ;[1 1 1] slow speed
  (set `CharacterMovementComponent.MaxWalkSpeed` (`self.slowSpeed`) (`Character.CharacterMovement` (`GameplayStatics.GetPlayerCharacter` 0)))
  (`KismetSystemLibrary.Delay` (`self.SlowDuration`))
  ;[1 1 1] normal speed
  (set `CharacterMovementComponent.MaxWalkSpeed` (`self.normalSpeed`) (`Character.CharacterMovement` (`GameplayStatics.GetPlayerCharacter` 0))))

(fn `UserConstructionScript`)