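; Garbage fountain hazard that kills the top-down player character on contact with its KillBox.
; On overlap it disables the character's input, stops movement immediately and calls its death function.
; Every Tick re-attaches the KillBox to the Snake component's HitBoxConnector socket, snapping its location to follow that point.
; A randomly delayed, looping Timeline meant to move and scale the sludge is disconnected and never runs.
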(event `self.ReceiveBeginPlay`
  ;[1 1 1] loops the scale and movement of the sludge "trash"
)

(event `self.killBox.OnComponentBeginOverlap`
  (params (OverlappedComponent :type "PrimitiveComponent Object Reference") (OtherActor :type "Actor Object Reference") (OtherComp :type "PrimitiveComponent Object Reference") (OtherBodyIndex :type Integer) (bFromSweep :type Boolean) (SweepResult :type "HitResult Structure (by ref)"))
  ;[1 1 1] death block
  (bind _asbp_top_down_character (cast `/Game/Blueprints/Player/BP_TopDownCharacter` OtherActor))
  (`self.DisableInput` _asbp_top_down_character null)
  (`MovementComponent.StopMovementImmediately` (`Character.CharacterMovement` _asbp_top_down_character))
  (`/Game/Blueprints/Player/BP_TopDownCharacter.Death` _asbp_top_down_character))

(event `self.ReceiveTick`
  (params (DeltaSeconds :type "Float (single-precision)"))
  (bind _snake (`self.Snake`))
  (`SceneComponent.K2_AttachToComponent` (`self.killBox`) _snake (`SkinnedMeshComponent.GetSocketBoneName` _snake "HitBoxConnector") "SnapToTarget" "KeepRelative" "KeepRelative" true))

(fn `sludgeHeightAdjuster`
  (returns (ReturnValue :type "Vector Structure")))

(fn `UserConstructionScript`)