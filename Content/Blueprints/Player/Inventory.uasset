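; Player inventory Blueprint that tracks pickup counts and upgrade ownership in two maps keyed by enum.
; Initialize seeds every pickup type with 10, despite its comment saying 0, and pickup, consume and custom changes route through InvPickupOrConsume.
; CreateUpgrade checks each DT_Upgrades recipe entry separately and toggles unowned upgrades on, but its item-deduction call is unwired.
; UseUpgrade removes an owned upgrade, only printing its effect.
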(event `Initialize`
  ;[0 0 0] Initialize the inventory with all pickup items with a count of 0
  (`BlueprintMapLibrary.Map_Clear` (`self.Item Inventory `))
  (bind _enumvalue (foreach `/Game/Blueprints/Pickups/E_Pickups` false)
    (:`LoopBody`
      (`BlueprintMapLibrary.Map_Add` (`self.Item Inventory `) _enumvalue 10)
      (`BlueprintMapLibrary.Map_Clear` (`self.Upgrade Inventory`)))))

(event `ModifyItemQuantity`
  (params (ItemName :type "/Game/Blueprints/Pickups/E_Pickups Enum" :default "NewEnumerator0") (Pickup :type Boolean))
  (bind _delta (`self.Delta`))
  ;[1 1 1] Item Pickup/Consumption inventory adjustment
  (if Pickup
    (set `self.Delta` 1)
    ;;[1 1 1] Picking up an Item
    (`self.InvPickupOrConsume` ItemName _delta)
    (else
      (set `self.Delta` -1)
      ;;[1 1 1] Consuming an Item
      (`self.InvPickupOrConsume` ItemName _delta))))

(event `CustomModify`
  (params (ItemName :type "/Game/Blueprints/Pickups/E_Pickups Enum" :default "NewEnumerator0") (Modifier :type Integer))
  (`self.InvPickupOrConsume` ItemName Modifier))

(event `UseUpgrade`
  (params (Upgrade :type "/Game/Blueprints/Pickups/E_Upgrades Enum (by ref)" :default "NewEnumerator0"))
  ;[1 1 1] Upgrade Use
  (if (`BlueprintMapLibrary.Map_Find` (`self.Upgrade Inventory`) Upgrade)
    (set `self.CanUse` true)
    (`KismetSystemLibrary.PrintString` (`KismetStringLibrary.Concat_StrStr` "Perform: " (`|GetEnumeratorNameAsString` Upgrade)))
    (`self.ToggleUpgradeInventoryStatus` Upgrade)
    (`BlueprintMapLibrary.Map_Remove` (`self.Upgrade Inventory`) Upgrade)
    (else
      (`KismetSystemLibrary.PrintString` "Nah dawg, you ain't got none of those")
      (set `self.CanUse` false))))

(event `CreateUpgrade`
  (params (Upgrade :type "/Game/Blueprints/Pickups/E_Upgrades Enum" :default "NewEnumerator0"))
  (bind _returnvalue (`KismetStringLibrary.Conv_StringToName` (`|GetEnumeratorNameAsString` Upgrade)))
  ;[1 1 1] Upgrade Creation
  ;;[0.5117 0.9741 1 1 12] Check if upgrade exists
  (bind _returnvalue_2 (`|GetDataTableRow` "/Game/Blueprints/Pickups/DT_Upgrades.DT_Upgrades" _returnvalue)
    (:`then`
      (bind ((`Type_28_00AEB10E42557BB3CFDCF4A39109AE01` _type) (`Recipe_9_CA52C2A74CBC861656DE4EBCFC868640` _recipe)) (break `/Game/Blueprints/Pickups/S_Recipes` _returnvalue_2))
      (bind (_key _value) (`/Game/Blueprints/HelperLibraries/HelperMacros.IterateMap (Pickup | Int)` _recipe)
        (:`LoopBody`
          (if (`BlueprintMapLibrary.Map_Contains` (`self.Item Inventory `) _key)
            (if (>= (`BlueprintMapLibrary.Map_Find` (`self.Item Inventory `) _key) _value)
              ;;[1 0.9302 0.5123 1 10] Subtract number of items used in recipe from inventory
              (bind _result (`/Engine/EditorBlueprintResources/StandardMacros.NegateInt` _value)
                (:`  `
                  (if (not (`.ReturnValue` (`BlueprintMapLibrary.Map_Find` (`self.Upgrade Inventory`) _type)))
                    (`self.ToggleUpgradeInventoryStatus` _type)
                    (else
                      (`KismetSystemLibrary.PrintString` (`KismetStringLibrary.Concat_StrStr` "Already in inventory, cannot create: " (`KismetStringLibrary.Conv_NameToString` _returnvalue)))))))
              (else
                (`KismetSystemLibrary.PrintString` (`KismetStringLibrary.Concat_StrStr` "Not enough items to create: " (`KismetStringLibrary.Conv_NameToString` _returnvalue)))))))))))