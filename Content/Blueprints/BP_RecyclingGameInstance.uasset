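; Game instance for the recycling game that opens the main menu, inventory, options and upgrades screens and starts play.
; Each Show event lazily creates and caches its widget, then adds it to the viewport.
; Main menu, inventory and upgrades also set a UI input mode and show the cursor, while options leaves both untouched.
; PlayGame opens Testing_Platform, switches to game-only input and hides the cursor.
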(event `ShowMainMenu`
  (bind _returnvalue (`GameplayStatics.GetPlayerController` 0))
  (bind _w_mainmenu (`self.W_MainMenu`))
  ;[0 0 0] Show the main menu
  (`/Engine/EditorBlueprintResources/StandardMacros.IsValid` (`self.W_MainMenu`)
    (:`Is Valid`
      _)
    (:`Is Not Valid`
      (bind _returnvalue_2 (`|CreateWidget` "/Game/Blueprints/UI/W_MainMenu.W_MainMenu_C"))
      (set `self.W_MainMenu` _returnvalue_2)))
  (`UserWidget.AddToViewport` _w_mainmenu 0)
  (`WidgetBlueprintLibrary.SetInputMode_GameAndUIEx` _returnvalue _w_mainmenu)
  (set `PlayerController.bShowMouseCursor` true _returnvalue))

(event `ShowInventory`
  (bind _returnvalue (`GameplayStatics.GetPlayerController` 0))
  ;[0 0 0] Show the main menu
  (`/Engine/EditorBlueprintResources/StandardMacros.IsValid` (`self.W_Inventory`)
    (:`Is Valid`
      _)
    (:`Is Not Valid`
      (bind _returnvalue_2 (`|CreateWidget` "/Game/Blueprints/UI/W_Inventory.W_Inventory_C"))
      (set `self.W_Inventory` _returnvalue_2)))
  (`UserWidget.AddToViewport` (`self.W_Inventory`) 0)
  (`WidgetBlueprintLibrary.SetInputMode_UIOnlyEx` _returnvalue null)
  (set `PlayerController.bShowMouseCursor` true _returnvalue))

(event `ShowOptionsMenu`
  ;[0 0 0] Show the main menu
  (`/Engine/EditorBlueprintResources/StandardMacros.IsValid` (`self.W_OptionsMenu`)
    (:`Is Valid`
      _)
    (:`Is Not Valid`
      (bind _returnvalue (`|CreateWidget` "/Game/Blueprints/UI/W_OptionsMenu.W_OptionsMenu_C"))
      (set `self.W_OptionsMenu` _returnvalue)))
  (`UserWidget.AddToViewport` (`self.W_OptionsMenu`) 0))

(event `ShowUpgrades`
  (bind _returnvalue (`GameplayStatics.GetPlayerController` 0))
  ;[0 0 0] Show the main menu
  (`/Engine/EditorBlueprintResources/StandardMacros.IsValid` (`self.W_Upgrades`)
    (:`Is Valid`
      _)
    (:`Is Not Valid`
      (bind _returnvalue_2 (`|CreateWidget` "/Game/Blueprints/UI/W_Upgrades.W_Upgrades_C"))
      (set `self.W_Upgrades` _returnvalue_2)))
  (`UserWidget.AddToViewport` (`self.W_Upgrades`) 0)
  (`WidgetBlueprintLibrary.SetInputMode_GameAndUIEx` _returnvalue null)
  (set `PlayerController.bShowMouseCursor` true _returnvalue))

(event `PlayGame`
  (bind _returnvalue (`GameplayStatics.GetPlayerController` 0))
  ;[0 0 0] Start playing the game with the users input focused on the game
  (`GameplayStatics.OpenLevel` "Testing_Platform" true "listen")
  (`WidgetBlueprintLibrary.SetInputMode_GameOnly` _returnvalue)
  (set `PlayerController.bShowMouseCursor` false _returnvalue))